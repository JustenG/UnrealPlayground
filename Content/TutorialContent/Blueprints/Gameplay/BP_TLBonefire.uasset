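; BP_TLBonefire is a bonfire save point that the player lights through a nearby interaction.
; Interacting sets FireActive, saves through TLGameModeBase's WriteSaveGame, reveals the fire particle system and prints a saved message.
; When the actor is loaded, OnActorLoaded shows the fire again if FireActive is set, so a lit bonfire stays lit.
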(event Custom|StartFire
  (Rendering|SetVisibility (Variables|Default|GetParticleSystem) true false))

(event EventBeginPlay)

(event Collision|EventActorBeginOverlap
  (params (OtherActor :type Actor%20Object%20Reference)))

(event EventTick
  (params (DeltaSeconds :type Float%20%28single-precision%29)))

(event EventInteract
  (params (InstigatorPawn :type Pawn%20Object%20Reference) (InteractionType :type ETLInteractionType%20Enum :default "EBT_INDIRECT"))
  (if (== InteractionType (Math|Conversions|ToInteger(Byte) (Utilities|Enum|LiteralenumETLInteractionType "EBT_NEARBY")))
    (Variables|Default|SetbFireActive true)
    (bind _astlgame_mode_base (Utilities|Casting|CastToTLGameModeBase (Game|GetGameMode)))
    (Class|TLGameModeBase|WriteSaveGame _astlgame_mode_base)
    (CallFunction|StartFire)
    (Development|PrintString "GAME SAVED")))

(event EventOnActorLoaded
  (if (Variables|Default|GetbFireActive)
    (CallFunction|StartFire)))

(fn ConstructionScript)