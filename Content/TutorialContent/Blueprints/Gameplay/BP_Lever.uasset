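; BP_Lever is an interactable lever that triggers another actor when used from nearby.
; A NEARBY Interact event snaps HandleMesh to a tilted rotation, then sets a second rotation after a short Delay.
; It then forwards an INDIRECT InteractMessage to OtherActor if one is set, chaining the interaction to that target.
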(event EventBeginPlay)

(event Collision|EventActorBeginOverlap
  (params (OtherActor :type Actor%20Object%20Reference)))

(event EventTick
  (params (DeltaSeconds :type Float%20%28single-precision%29)))

(event EventInteract
  (params (InstigatorPawn :type Pawn%20Object%20Reference) (InteractionType :type ETLInteractionType%20Enum :default "EBT_INDIRECT"))
  (if (== InteractionType (Math|Conversions|ToInteger(Byte) (Utilities|Enum|LiteralenumETLInteractionType "EBT_NEARBY")))
    (Transformation|SetRelativeRotation (Variables|Default|GetHandleMesh) (Math|Rotator|MakeRotator 0.0 -3e+01 0.0) false false)
    (Utilities|FlowControl|Delay 1.0)
    (Transformation|SetRelativeRotation (Variables|Default|GetHandleMesh) "30.000000,0.000000,0.000000" false false)
    (if (!= (Variables|Default|GetOtherActor) 0)
      (Class|TLGameplayInterface|Interact(Message) (Variables|Default|GetOtherActor) 0 "EBT_INDIRECT"))))

(fn ConstructionScript)