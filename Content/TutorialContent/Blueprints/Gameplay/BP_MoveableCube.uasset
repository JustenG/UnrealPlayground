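; Tutorial cube actor that slides from its starting position to EndVector when triggered by an indirect interaction, with a camera shake during the move.
; Interact sets Moving and starts the shake; Tick advances Delta by MoveMag per second and lerps the cube's relative location.
; Movement ends once Delta reaches 1 and is never reset; Tick stops all shakes whenever idle.
; CanInteract always returns false.
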(event EventBeginPlay
  (Variables|Default|SetStartVector (Variables|/Script/Engine.SceneComponent|GetRelativeLocation (Variables|Default|GetCube))))

(event Collision|EventActorBeginOverlap
  (params (OtherActor :type Actor%20Object%20Reference)))

(event EventTick
  (params (DeltaSeconds :type Float%20%28single-precision%29))
  (if (Variables|Default|GetMoving)
    (Variables|Default|SetDelta (+ (* (Variables|Default|GetMoveMag) DeltaSeconds) (Variables|Default|GetDelta)))
    (bind _output_get (Variables|Default|SetResultVector (Math|Vector|Lerp(Vector) (Variables|Default|GetStartVector) (Variables|Default|GetEndVector) (Variables|Default|GetDelta))))
    (Transformation|SetRelativeLocation (Variables|Default|GetCube) _output_get false false)
    (Variables|Default|SetMoving (< (Variables|Default|GetDelta) 1.0))
    (else
      (CameraShake|StopAllCameraShakes (Variables|Default|GetCameraShakeSource) true))))

(event EventInteract
  (params (InstigatorPawn :type Pawn%20Object%20Reference) (InteractionType :type ETLInteractionType%20Enum :default "EBT_INDIRECT"))
  (if (== InteractionType (Math|Conversions|ToInteger(Byte) (Utilities|Enum|LiteralenumETLInteractionType "EBT_INDIRECT")))
    (Variables|Default|SetMoving true)
    (CameraShakes|StartCameraShake (Variables|Default|GetCameraShakeSource) "/Game/ExampleContent/CameraShake/camera_shake_constant.camera_shake_constant_C" 1.0 "CameraLocal" "0, 0, 0")))

(fn ConstructionScript)

(fn CanInteract
  (params (InstigatorPawn :type Pawn%20Object%20Reference) (InteractionType :type ETLInteractionType%20Enum :default "EBT_INDIRECT"))
  (return false))